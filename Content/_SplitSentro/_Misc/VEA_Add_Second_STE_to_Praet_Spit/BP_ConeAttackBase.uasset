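; Mod hook on BP_ConeAttackBase that adds a plasma carbine Conductive Thermals status effect to cone attacks owned by ENE_Shredder_Base.
; Hooked begin and end overlap handlers call the original stubs, then push or pop the effect on the other actor, skipping self.
; The owner check is an exact class match, despite the folder name referring to Praetorian spit.
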(fn HookConeBeginOverlap
  (params (OverlappedComponent :type Primitive%20Component%20Object%20Reference) (OtherActor :type Actor%20Object%20Reference) (OtherComp :type Primitive%20Component%20Object%20Reference) (OtherBodyIndex :type Integer) (bFromSweep :type Boolean) (SweepResult :type Hit%20Result%20Structure))
  (CallFunction|OrigConeBeginOverlap OverlappedComponent OtherActor OtherComp OtherBodyIndex bFromSweep SweepResult)
  (if (!= OtherActor self)
    (if (== (Utilities|GetClass (Components|GetOwner)) "/Game/Enemies/RivalTech/Shredder/ENE_Shredder_Base.ENE_Shredder_Base_C")
      (Class|StatusEffectsComponent|TryPushActiveStatusEffect "/Game/WeaponsNTools/PlasmaCarbine/STE_ConductiveTermals_PlasmaCarbine.STE_ConductiveTermals_PlasmaCarbine_C" OtherActor (Components|GetOwner)))))

(fn OrigConeBeginOverlap
  (params (OverlappedComponent :type Primitive%20Component%20Object%20Reference) (OtherActor :type Actor%20Object%20Reference) (OtherComp :type Primitive%20Component%20Object%20Reference) (OtherBodyIndex :type Integer) (bFromSweep :type Boolean) (SweepResult :type Hit%20Result%20Structure)))

(fn HookConeEndOverlap
  (params (OverlappedComponent :type Primitive%20Component%20Object%20Reference) (OtherActor :type Actor%20Object%20Reference) (OtherComp :type Primitive%20Component%20Object%20Reference) (OtherBodyIndex :type Integer))
  (CallFunction|OrigConeEndOverlap OverlappedComponent OtherActor OtherComp OtherBodyIndex)
  (if (!= OtherActor self)
    (if (== (Utilities|GetClass (Components|GetOwner)) "/Game/Enemies/RivalTech/Shredder/ENE_Shredder_Base.ENE_Shredder_Base_C")
      (Class|StatusEffectsComponent|TryPopActiveStatusEffect "/Game/WeaponsNTools/PlasmaCarbine/STE_ConductiveTermals_PlasmaCarbine.STE_ConductiveTermals_PlasmaCarbine_C" OtherActor (Components|GetOwner)))))

(fn OrigConeEndOverlap
  (params (OverlappedComponent :type Primitive%20Component%20Object%20Reference) (OtherActor :type Actor%20Object%20Reference) (OtherComp :type Primitive%20Component%20Object%20Reference) (OtherBodyIndex :type Integer)))