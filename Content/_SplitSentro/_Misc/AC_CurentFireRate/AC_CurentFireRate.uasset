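; AC_CurentFireRate is a debug helper that shows the Autocannon's current rate of fire in a watch under the Weapons category.
; On BeginPlay it polls every second until the last AutoCannon actor found is valid, then adds a watch fed by that weapon's CurrentFireTime.
; It also binds to the first player's character-spawned event, apparently to repeat the search and watch setup after a delay for the new weapon.
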(event Custom|WATCH
  (params (ValueHolder :type LIB%20DEB%20O%20Value%20Holder%20Object%20Reference))
  ;[0 0 1] AC_CurentFireRate: watch Autocannon's Rate of Fire.
  (Default|SetValue ValueHolder (Utilities|String|ToString(Float) (Variables|/Script/FSD.AutoCannon|GetCurrentFireTime (Variables|Default|GetAutocannon)))))

(event Custom|RESET_WATCH
  (params (PlayerCharacter :type Player%20Character%20Object%20Reference))
  ;[0 0 1] AC_CurentFireRate: watch Autocannon's Rate of Fire.
  (Utilities|FlowControl|Delay 1.0) ; Waiting for the new Autocannon to spawn\nafter the Character spawn event.
  (bind _outactors (Actor|GetAllActorsOfClass "/Script/FSD.AutoCannon" :!label _label))
  (Utilities|IsValid (Utilities|Array|Get(acopy) _outactors (Utilities|Array|LastIndex _outactors))
    (:Is%20Valid
      (Variables|Default|SetAutocannon (Utilities|Array|Get(acopy) _outactors (Utilities|Array|LastIndex _outactors)))
      (bind _createdvalueholder (CallFunction|AddDebugWatch :WatchDisplayName "Autocannon RoF" :Category (Utilities|Array|MakeArray "Weapons") :Description "Curent rate of fire of Autocannon" :VariableTypeColor "NewEnumerator3"))
      (EventDispatchers|BindEventtoRequestNewValue _createdvalueholder (delegate Custom|WATCH))
      (bind _asfsdplayer_state (Utilities|Casting|CastToFSDPlayerState (Variables|/Script/Engine.Controller|GetPlayerState (Class|GameplayStatics|GetPlayerControllerfromID))))
      (EventDispatchers|BindEventtoOnPlayerCharacterSpawned _asfsdplayer_state (EventDispatchers|CreateEvent :!event Custom|RESET_WATCH)))
    (:Is%20Not%20Valid
      (Utilities|FlowControl|Delay 1.0)
      (goto _label))))

(event EventBeginPlay
  ;[0 0 1] AC_CurentFireRate: watch Autocannon's Rate of Fire.
  (bind _outactors (Actor|GetAllActorsOfClass "/Script/FSD.AutoCannon" :!label _label))
  (Utilities|IsValid (Utilities|Array|Get(acopy) _outactors (Utilities|Array|LastIndex _outactors))
    (:Is%20Valid
      (Variables|Default|SetAutocannon (Utilities|Array|Get(acopy) _outactors (Utilities|Array|LastIndex _outactors)))
      (bind _createdvalueholder (CallFunction|AddDebugWatch :WatchDisplayName "Autocannon RoF" :Category (Utilities|Array|MakeArray "Weapons") :Description "Curent rate of fire of Autocannon" :VariableTypeColor "NewEnumerator3"))
      (EventDispatchers|BindEventtoRequestNewValue _createdvalueholder (delegate Custom|WATCH))
      (bind _asfsdplayer_state (Utilities|Casting|CastToFSDPlayerState (Variables|/Script/Engine.Controller|GetPlayerState (Class|GameplayStatics|GetPlayerControllerfromID))))
      (EventDispatchers|BindEventtoOnPlayerCharacterSpawned _asfsdplayer_state (EventDispatchers|CreateEvent :!event Custom|RESET_WATCH)))
    (:Is%20Not%20Valid
      (Utilities|FlowControl|Delay 1.0)
      (goto _label))))

(fn ConstructionScript)