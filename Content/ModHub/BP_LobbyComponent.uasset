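; Lobby component from ModHub that overrides the game's max player count to a preferred lobby size.
; Once enabled on the server, a looping timer re-applies the cap through FSDGameInstance, and preference changes apply immediately.
; The preference is clamped to 1–7 on the Space Rig or while a landing drop pod exists, and is unclamped otherwise.
; Listeners are notified on enabling and on size changes.
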(event Custom|EnableLobbyFeatures
  (params (MaxPlayersPreference :type Integer))
  (if (Networking|IsServer)
    (if (not (Variables|Default|GetIsLobbyFeaturesEnabled))
      (Variables|Default|SetIsLobbyFeaturesEnabled true)
      (Variables|Default|SetMaxPlayersPreference MaxPlayersPreference)
      (bind _returnvalue (Utilities|Time|SetTimerbyEvent (delegate Custom|UpdatePlayerCap) 5.0 true))
      (Variables|Default|SetLobbyCheckTimer _returnvalue)
      (CallFunction|UpdatePlayerCap)
      (bind _returnvalue_2 (CallFunction|GetMaxPlayerCount))
      (Default|CallOnLobbySizeChanged _returnvalue_2)
      (Default|CallOnLobbyFeaturesEnabled))))

(event Custom|UpdatePlayerCap
  (if (CallFunction|IsLobbySpacerig)
    (CallFunction|SetMaxPlayerCount (Math|Integer|Clamp(Integer) (Variables|Default|GetMaxPlayersPreference) 1 7) false)
    (else
      (bind _outactors (Actor|GetAllActorsOfClass "/Game/LevelElements/Droppod/BP_DropPod_Landing.BP_DropPod_Landing_C"))
      (if (> (Utilities|Array|Length _outactors) 0)
        (CallFunction|SetMaxPlayerCount (Math|Integer|Clamp(Integer) (Variables|Default|GetMaxPlayersPreference) 1 7) false)
        (else
          (CallFunction|SetMaxPlayerCount (Variables|Default|GetMaxPlayersPreference) false))))))

(fn SetMaxPlayersPreference
  (params (MaxLobbySize :type Integer))
  (Variables|Default|SetMaxPlayersPreference MaxLobbySize)
  (if (Variables|Default|GetIsLobbyFeaturesEnabled)
    (CallFunction|UpdatePlayerCap)))

(fn IsLobbySpacerig
  (bind _returnvalue (Game|GetCurrentLevelName true))
  (return (Utilities|Enum|Equal(Enum) _returnvalue "LVL_SpaceRig")))

(fn GetMaxPlayerCount
  (bind _asfsdgame_instance (Utilities|Casting|CastToFSDGameInstance (Game|GetGameInstance)))
  (return (Class|FSDGameInstance|GetOverrideMaxPlayerCount _asfsdgame_instance)))

(fn SetMaxPlayerCount
  (params (Count :type Integer) (ForceUpdate :type Boolean))
  (bind _returnvalue (CallFunction|GetMaxPlayerCount))
  (if (or (!= _returnvalue Count) ForceUpdate)
    (bind _asfsdgame_instance (Utilities|Casting|CastToFSDGameInstance (Game|GetGameInstance)))
    (Class|FSDGameInstance|SetOverrideMaxPlayerCount _asfsdgame_instance Count)
    (Default|CallOnLobbySizeChanged Count)))